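; BP_Suiti_B is a switch actor that opens BP_Door_B while a player stands in its Box trigger.
; A BP_PlayerBass overlap swaps the Suiti material, sets IsActive and calls OpenDoor, gated by a DoOnce.
; Any player's exit restores the material, calls NotOpenDoor and resets the DoOnce, without checking for remaining players.
; BeginPlay caches BP_Door_A and all players, but the overlap logic uses neither.
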(event OnComponentBeginOverlap(Box)
  (params (OverlappedComponent :type Primitive%20Component%20Object%20Reference) (OtherActor :type Actor%20Object%20Reference) (OtherComp :type Primitive%20Component%20Object%20Reference) (OtherBodyIndex :type Integer) (bFromSweep :type Boolean) (SweepResult :type Hit%20Result%20Structure%20%28by%20ref%29))
  (bind _asbp_player_bass (Utilities|Casting|CastToBP_PlayerBass OtherActor))
  (Variables|Default|SetAs%20BP%20Player%20Bass_0 _asbp_player_bass)
  (Utilities|FlowControl|DoOnce false
    (:Completed
      (if (not (Variables|Default|GetIs%20Active?))
        (Rendering|Material|SetMaterial (Variables|Default|GetSuiti) 0 "/Engine/VREditor/BasicMeshes/MI_Cube_03.MI_Cube_03")
        (Variables|Default|SetIs%20Active? true)
        (bind _returnvalue (Actor|GetActorOfClass "/Game/Gimiku/BP_Gimiku/Door/BP_Door_B.BP_Door_B_C"))
        (Default|OpenDoor _returnvalue)))))

(event OnComponentEndOverlap(Box)
  (params (OverlappedComponent :type Primitive%20Component%20Object%20Reference) (OtherActor :type Actor%20Object%20Reference) (OtherComp :type Primitive%20Component%20Object%20Reference) (OtherBodyIndex :type Integer))
  (Utilities|Casting|CastToBP_PlayerBass OtherActor)
  (Utilities|FlowControl|Sequence
    (:then_0
      (Rendering|Material|SetMaterial (Variables|Default|GetSuiti) 0 "/Engine/BasicShapes/BasicShapeMaterial.BasicShapeMaterial")
      (Variables|Default|SetIs%20Active? false)
      (bind _returnvalue (Actor|GetActorOfClass "/Game/Gimiku/BP_Gimiku/Door/BP_Door_B.BP_Door_B_C"))
      (Default|NotOpenDoor _returnvalue))
    (:then_1
      (Utilities|FlowControl|DoOnce false) ; enters at Reset
    )))

(event EventBeginPlay
  (bind _returnvalue (Actor|GetActorOfClass "/Game/Gimiku/BP_Gimiku/Door/BP_Door_A.BP_Door_A_C"))
  (Variables|Default|SetNewVar _returnvalue)
  (bind _outactors (Actor|GetAllActorsOfClass "/Game/hibiki/BP_PlayerBass.BP_PlayerBass_C"))
  (Variables|Default|SetALL_Player _outactors))

(fn ConstructionScript)