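; BP_Suiti is a one-shot switch gimmick that opens a door when the player touches it.
; A Box overlap by player character 0 swaps the Suiti component's material to MI_Cube_03 and sets IsActive, blocking retriggering.
; It then calls OpenDoor on the BP_Door returned by GetActorOfClass, so it targets the first door found rather than an assigned reference.
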(event OnComponentBeginOverlap(Box)
  (params (OverlappedComponent :type Primitive%20Component%20Object%20Reference) (OtherActor :type Actor%20Object%20Reference) (OtherComp :type Primitive%20Component%20Object%20Reference) (OtherBodyIndex :type Integer) (bFromSweep :type Boolean) (SweepResult :type Hit%20Result%20Structure%20%28by%20ref%29))
  (if (and (== OtherActor (Game|GetPlayerCharacter 0)) (not (Variables|Default|GetIs%20Active?)))
    (Rendering|Material|SetMaterial (Variables|Default|GetSuiti) 0 "/Engine/VREditor/BasicMeshes/MI_Cube_03.MI_Cube_03")
    (Variables|Default|SetIs%20Active? true)
    (bind _returnvalue (Actor|GetActorOfClass "/Game/Gimiku/BP_Gimiku/BP_Door.BP_Door_C"))
    (Default|OpenDoor _returnvalue)))

(event EventBeginPlay)

(event Collision|EventActorBeginOverlap
  (params (OtherActor :type Actor%20Object%20Reference)))

(event EventTick
  (params (DeltaSeconds :type Float%20%28single-precision%29)))

(fn ConstructionScript)