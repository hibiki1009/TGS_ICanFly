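; Speed-up floor gimmick that boosts player walk speed while a BP_PlayerBass is inside its Box trigger.
; Begin overlap spawns the UpSpeed particle at that player and adds a fixed amount to MaxWalkSpeed; end overlap subtracts it.
; Both changes apply to player characters 0 and 1 together, whichever one overlapped, and build on the current GetMaxSpeed rather than a stored base speed.
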(event OnComponentBeginOverlap(Box)
  (params (OverlappedComponent :type Primitive%20Component%20Object%20Reference) (OtherActor :type Actor%20Object%20Reference) (OtherComp :type Primitive%20Component%20Object%20Reference) (OtherBodyIndex :type Integer) (bFromSweep :type Boolean) (SweepResult :type Hit%20Result%20Structure%20%28by%20ref%29))
  (bind _returnvalue (Game|GetPlayerCharacter 1))
  (bind _returnvalue_2 (Game|GetPlayerCharacter 0))
  (bind _charactermovement (Variables|/Script/Engine.Character|GetCharacterMovement _returnvalue_2))
  (bind _charactermovement_2 (Variables|/Script/Engine.Character|GetCharacterMovement _returnvalue))
  (bind _asbp_player_bass (Utilities|Casting|CastToBP_PlayerBass OtherActor))
  (Effects|SpawnEmitteratLocation "/Game/Effect/UpSpeed.UpSpeed" (Transformation|GetActorLocation _asbp_player_bass))
  (Utilities|FlowControl|Sequence
    (:then_0
      (Variables|/Script/Engine.CharacterMovementComponent|SetMaxWalkSpeed _charactermovement (+ (Class|MovementComponent|GetMaxSpeed _charactermovement) 2e+02)))
    (:then_1
      (Variables|/Script/Engine.CharacterMovementComponent|SetMaxWalkSpeed _charactermovement_2 (+ (Class|MovementComponent|GetMaxSpeed _charactermovement_2) 2e+02)))))

(event OnComponentEndOverlap(Box)
  (params (OverlappedComponent :type Primitive%20Component%20Object%20Reference) (OtherActor :type Actor%20Object%20Reference) (OtherComp :type Primitive%20Component%20Object%20Reference) (OtherBodyIndex :type Integer))
  (bind _returnvalue (Game|GetPlayerCharacter 0))
  (bind _returnvalue_2 (Game|GetPlayerCharacter 1))
  (bind _charactermovement (Variables|/Script/Engine.Character|GetCharacterMovement _returnvalue))
  (bind _charactermovement_2 (Variables|/Script/Engine.Character|GetCharacterMovement _returnvalue_2))
  (Utilities|Casting|CastToBP_PlayerBass OtherActor)
  (Utilities|FlowControl|Sequence
    (:then_0
      (Variables|/Script/Engine.CharacterMovementComponent|SetMaxWalkSpeed _charactermovement (- (Class|MovementComponent|GetMaxSpeed _charactermovement) 2e+02)))
    (:then_1
      (Variables|/Script/Engine.CharacterMovementComponent|SetMaxWalkSpeed _charactermovement_2 (- (Class|MovementComponent|GetMaxSpeed _charactermovement_2) 2e+02)))))

(event EventBeginPlay)

(event Collision|EventActorBeginOverlap
  (params (OtherActor :type Actor%20Object%20Reference)))

(event EventTick
  (params (DeltaSeconds :type Float%20%28single-precision%29)))

(fn ConstructionScript)