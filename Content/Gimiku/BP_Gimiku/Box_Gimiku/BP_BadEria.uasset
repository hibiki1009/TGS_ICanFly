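; BP_BadEria is a gimmick trigger volume that sends both local players back to a target point when a BP_PlayerBass enters it.
; On overlap it creates a WI_BadEria widget and plays its Fadeout animation.
; It immediately teleports player 1 to TeleportTarget and player 0 to the same spot shifted by a fixed X offset, regardless of which player triggered it.
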(event OnComponentBeginOverlap(BadEria)
  (params (OverlappedComponent :type Primitive%20Component%20Object%20Reference) (OtherActor :type Actor%20Object%20Reference) (OtherComp :type Primitive%20Component%20Object%20Reference) (OtherBodyIndex :type Integer) (bFromSweep :type Boolean) (SweepResult :type Hit%20Result%20Structure%20%28by%20ref%29))
  (bind _teleporttarget (Variables|Default|GetTeleportTarget))
  (bind _returnvalue (Transformation|GetActorLocation _teleporttarget))
  (Utilities|Casting|CastToBP_PlayerBass OtherActor)
  (bind _returnvalue_2 (UserInterface|CreateWidget "/Game/Gimiku/WI_BadEria.WI_BadEria_C"))
  (UserInterface|Viewport|AddtoViewport _returnvalue_2 0)
  (UserInterface|Animation|PlayAnimation _returnvalue_2 (Variables|/Game/Gimiku/WI_BadEria.WI_BadEria_C|GetFadeout _returnvalue_2) 0.0 1 "Forward" 1.0 false)
  (Transformation|SetActorLocation (Game|GetPlayerCharacter 1) (Transformation|GetActorLocation (Variables|Default|GetTeleportTarget)) false true)
  (Transformation|SetActorLocation (Game|GetPlayerCharacter 0) (Math|Vector|MakeVector (+ (.x (Transformation|GetActorLocation (Variables|Default|GetTeleportTarget))) 1131.0) (.y _returnvalue) (.z _returnvalue)) false true))

(event EventBeginPlay)

(event Collision|EventActorBeginOverlap
  (params (OtherActor :type Actor%20Object%20Reference)))

(event EventTick
  (params (DeltaSeconds :type Float%20%28single-precision%29)))

(fn ConstructionScript)