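; Gimmick door that slides vertically open once at least three switches are active and closes when the count drops below that.
; Open_Door and Not_Open_Door raise and lower the ActiveSwitch counter, playing or reversing the Door_Open timeline at the threshold.
; The timeline offsets the door's world Z from the location saved at BeginPlay.
; A second timeline that sets relative location is left unconnected.
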(event Custom|Open_Door
  (bind _door (Variables|Default|GetDoor))
  (bind _returnvalue (Transformation|GetWorldLocation _door))
  (bind _result (Math|Integer|IncrementInt (Variables|Default|GetActiveSwitch))
    (:%20%20
      (if (> _result 2)
        (bind _open (Timeline|Door_Open Play)
          (:Update
            (Transformation|SetWorldLocation (Variables|Default|GetDoor) (Math|Vector|MakeVector (.x _returnvalue) (.y _returnvalue) (+ _open (.z (Variables|Default|GetStart_Location)))) false false)))))))

(event Custom|Not_Open_Door
  (bind _door (Variables|Default|GetDoor))
  (bind _returnvalue (Transformation|GetWorldLocation _door))
  (bind _result (Math|Integer|DecrementInt (Variables|Default|GetActiveSwitch))
    (:%20%20
      (if (< _result 3)
        (bind _open (Timeline|Door_Open Reverse)
          (:Update
            (Transformation|SetWorldLocation (Variables|Default|GetDoor) (Math|Vector|MakeVector (.x _returnvalue) (.y _returnvalue) (+ _open (.z (Variables|Default|GetStart_Location)))) false false)))))))

(event EventBeginPlay
  (Variables|Default|SetStart_Location (Transformation|GetWorldLocation (Variables|Default|GetDoor))))

(fn ConstructionScript)