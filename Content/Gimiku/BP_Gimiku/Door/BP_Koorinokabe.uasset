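; BP_Koorinokabe is an ice wall gimmick that melts once when the player touches it.
; On BeginPlay it creates a dynamic instance of M_Koori on the Kori mesh.
; The first overlap with a BP_PlayerBass plays the Tokeru (melt) timeline, which drives the material's Rate parameter.
; When the timeline finishes, it destroys the Hantei collision component while the actor itself remains.
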(event EventBeginPlay
  (bind _returnvalue (Rendering|Material|CreateDynamicMaterialInstance (Variables|Default|GetKori) 0 "/Game/Gimiku/BP_Gimiku/Material/M_Koori.M_Koori" "None" :!class /Script/Engine.PrimitiveComponent))
  (Variables|Default|SetM_1 _returnvalue))

(event EventTick
  (params (DeltaSeconds :type Float%20%28single-precision%29)))

(event Collision|EventActorBeginOverlap
  (params (OtherActor :type Actor%20Object%20Reference))
  (Utilities|Casting|CastToBP_PlayerBass OtherActor)
  (Utilities|FlowControl|DoOnce false
    (:Completed
      (bind _tokeru (Timeline|Tokeru Play)
        (:Update
          (Rendering|Material|SetScalarParameterValue (Variables|Default|GetM_1) "Rate" _tokeru :!class /Script/Engine.MaterialInstanceDynamic))
        (:Finished
          (Components|DestroyComponent (Variables|Default|GetHantei)))))))

(fn ConstructionScript)