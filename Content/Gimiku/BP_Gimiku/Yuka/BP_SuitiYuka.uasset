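; BP_SuitiYuka is a gimmick actor combining a pressure switch with a Door mesh that rises while switches are active.
; Player overlap on Box swaps the Suitti material and calls UpYuka or DownYuka on the first BP_SuitiYuka found by GetActorOfClass, not necessarily itself.
; That instance counts active switches in ActiveSwitch, playing a timeline to lift Door from its starting height and reversing it when none remain.
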(event OnComponentBeginOverlap(Box)
  (params (OverlappedComponent :type Primitive%20Component%20Object%20Reference) (OtherActor :type Actor%20Object%20Reference) (OtherComp :type Primitive%20Component%20Object%20Reference) (OtherBodyIndex :type Integer) (bFromSweep :type Boolean) (SweepResult :type Hit%20Result%20Structure%20%28by%20ref%29))
  (Utilities|FlowControl|DoOnce false
    (:Completed
      (Utilities|Casting|CastToBP_PlayerBass OtherActor)
      (if (not (Variables|Default|GetIs%20Active?))
        (Rendering|Material|SetMaterial (Variables|Default|GetSuitti) 0 "/Engine/VREditor/BasicMeshes/MI_Cube_03.MI_Cube_03")
        (Variables|Default|SetIs%20Active? true)
        (bind _returnvalue (Actor|GetActorOfClass "BP_SuitiYuka_C"))
        (CallFunction|UpYuka _returnvalue)))))

(event OnComponentEndOverlap(Box)
  (params (OverlappedComponent :type Primitive%20Component%20Object%20Reference) (OtherActor :type Actor%20Object%20Reference) (OtherComp :type Primitive%20Component%20Object%20Reference) (OtherBodyIndex :type Integer))
  (Utilities|FlowControl|Sequence
    (:then_0
      (Utilities|Casting|CastToBP_PlayerBass OtherActor)
      (Rendering|Material|SetMaterial (Variables|Default|GetSuitti) 0 "/Engine/BasicShapes/BasicShapeMaterial.BasicShapeMaterial")
      (Variables|Default|SetIs%20Active? false)
      (bind _returnvalue (Actor|GetActorOfClass "BP_SuitiYuka_C"))
      (CallFunction|DownYuka _returnvalue))
    (:then_1
      (Utilities|FlowControl|DoOnce false) ; enters at Reset
    )))

(event Custom|UpYuka
  (bind _door (Variables|Default|GetDoor))
  (bind _returnvalue (Transformation|GetWorldLocation _door))
  (bind _result (Math|Integer|IncrementInt (Variables|Default|GetActiveSwitch))
    (:%20%20
      (if (> _result 0)
        (bind _open (Timeline|タイムライン_0 Play)
          (:Update
            (Transformation|SetWorldLocation (Variables|Default|GetDoor) (Math|Vector|MakeVector (.x _returnvalue) (.y _returnvalue) (+ _open (.z (Variables|Default|GetStart_Location)))) false false)))))))

(event Custom|DownYuka
  (bind _door (Variables|Default|GetDoor))
  (bind _returnvalue (Transformation|GetWorldLocation _door))
  (bind _result (Math|Integer|DecrementInt (Variables|Default|GetActiveSwitch))
    (:%20%20
      (if (< _result 1)
        (bind _open (Timeline|タイムライン_0 Reverse)
          (:Update
            (Transformation|SetWorldLocation (Variables|Default|GetDoor) (Math|Vector|MakeVector (.x _returnvalue) (.y _returnvalue) (+ _open (.z (Variables|Default|GetStart_Location)))) false false)))))))

(event EventBeginPlay
  (Variables|Default|SetStart_Location (Transformation|GetWorldLocation (Variables|Default|GetDoor))))

(fn ConstructionScript)