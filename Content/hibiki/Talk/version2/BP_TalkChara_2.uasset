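; Talk character Blueprint that shows dialogue from DT_TalkData through a WBP_MessageWindow_2 widget.
; BeginPlay creates the widget and hands it the data table, and the Talk event adds it to the viewport and starts the conversation.
; Its own paging functions look like leftovers: nothing here calls CheckLastPage or ShowNextPage, LoadTalkData's row-reading logic is disconnected, and Talkread is empty.
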(event Custom|Talk
  (bind _messagewindow (Variables|Default|GetMessageWindow))
  (UserInterface|Viewport|AddtoViewport _messagewindow 0)
  (Default|TalkStart _messagewindow))

(event Custom|Talkread)

(event EventBeginPlay
  (bind _returnvalue (UserInterface|CreateWidget "/Game/hibiki/Talk/version2/WBP_MessageWindow_2.WBP_MessageWindow_2_C"))
  (bind _output_get (Variables|Default|SetMessageWindow _returnvalue))
  (Default|SetDataTable _output_get "/Game/hibiki/Talk/Talkdata/DT_TalkData.DT_TalkData"))

(fn ConstructionScript)

(fn CheckLastPage
  (params (Table :type Data%20Table%20Object%20Reference))
  (bind _outrownames (DataTable|GetDataTableRowNames Table))
  (for _array_element _outrownames
    (Math|Integer|IncrementInt (Variables|Default|GetLastPage))))

(fn LoadTalkData
  (params (DataTable :type Data%20Table%20Object%20Reference)))

(fn ShowNextPage
  (params (DataTable :type Data%20Table%20Object%20Reference))
  (if (Variables|Default|Getis_ShawMessage) ; widgetが表示されているかどうか
    (Math|Integer|IncrementInt (Variables|Default|GetCurrentPage)
      (:%20%20
        (if (> (Variables|Default|GetCurrentPage) (Variables|Default|GetLastPage)) ; ページ数がラストをこえたかどうか
          (Variables|Default|SetCurrentPage 1) ; 初めのページに戻す
          (Variables|Default|Setis_ShawMessage false)
          (else
            (CallFunction|LoadTalkData DataTable)))))))